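; Gameplay ability for a projectile spell that casts a firebolt toward the point under the mouse.
; On activation it gets target data under the mouse, turns the avatar to that point through CombatInterface and plays the cast montage.
; A montage gameplay event times the projectile spawn, after which the ability commits only its cooldown and ends.
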(event Ability|EventActivateAbility
  (bind _datahandle (|TargetDataUnderMouse)
    (:ValidData
      (bind _output_get (Variables|Default|SetProjectileLocation (.Location (Collision|BreakHitResult (Ability|TargetData|GetHitResultfromTargetData _datahandle)))))
      (bind _ascombat_interface (Utilities|Casting|CastToCombatInterface (Ability|GetAvatarActorfromActorInfo)))
      (Class|CombatInterface|UpdateFacingTarget _ascombat_interface _output_get)
      (|PlayMontageandWaitProxy "None" "/Game/Assets/Characters/Aura/Animations/Abilities/Cast_FireBolt_Montage.Cast_FireBolt_Montage" 1.0 "None" true 1.0 0.0 false
        (:then
          (Ability|Tasks|WaitGameplayEvent "(TagName=\"Event.Montage.FireBolt\")" 0
            (:EventReceived
              (Class|AuraProjectileSpell|SpawnProjectile _output_get)
              (Ability|CommitAbilityCooldown false)
              (Ability|EndAbility))))))))