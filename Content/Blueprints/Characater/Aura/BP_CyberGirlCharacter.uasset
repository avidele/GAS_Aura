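; Cyber girl character Blueprint that handles melee attack hit effects through left and right weapon collision components.
; StartAttack only unhides both weapon collisions in game; nothing here hides them again or changes their collision.
; Overlaps on either weapon spawn an attached Niagara fire explosion, but only the right one also applies the GE_TakeDamage gameplay effect to the other actor.
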(event OnComponentBeginOverlap(R_WeaponCollision)
  (params (OverlappedComponent :type Primitive%20Component%20Object%20Reference) (OtherActor :type Actor%20Object%20Reference) (OtherComp :type Primitive%20Component%20Object%20Reference) (OtherBodyIndex :type Integer) (bFromSweep :type Boolean) (SweepResult :type Hit%20Result%20Structure%20%28by%20ref%29))
  (Niagara|SpawnSystemAttached "/Game/Assets/Effects/Projectiles/FireExplosion/NS_FireExplosion.NS_FireExplosion" OverlappedComponent "None" "0, 0, 0" "0, 0, 0" "KeepRelativeOffset" false)
  (Class|AuraCharacterBase|ApplyEffecttoTarget OtherActor "/Game/Blueprints/Characater/Enemy/GE_TakeDamage.GE_TakeDamage_C" 1.0))

(event OnComponentBeginOverlap(L_WeaponCollision)
  (params (OverlappedComponent :type Primitive%20Component%20Object%20Reference) (OtherActor :type Actor%20Object%20Reference) (OtherComp :type Primitive%20Component%20Object%20Reference) (OtherBodyIndex :type Integer) (bFromSweep :type Boolean) (SweepResult :type Hit%20Result%20Structure%20%28by%20ref%29))
  (Niagara|SpawnSystemAttached "/Game/Assets/Effects/Projectiles/FireExplosion/NS_FireExplosion.NS_FireExplosion" OverlappedComponent "None" "0, 0, 0" "0, 0, 0" "KeepRelativeOffset" false))

(event Custom|StartAttack
  (Development|SetHiddeninGame (Variables|Default|GetR_WeaponCollision) false false)
  (Development|SetHiddeninGame (Variables|Default|GetL_WeaponCollision) false false))

(event EventBeginPlay
  (|CallParentFunction) ; This node is disabled and will not be called.\nDrag off pins to build functionality.
)

(event Collision|EventActorBeginOverlap
  (params (OtherActor :type Actor%20Object%20Reference))
  (|CallParentFunction OtherActor) ; This node is disabled and will not be called.\nDrag off pins to build functionality.
)

(event EventTick
  (params (DeltaSeconds :type Float%20%28single-precision%29))
  (|CallParentFunction DeltaSeconds) ; This node is disabled and will not be called.\nDrag off pins to build functionality.
)

(fn ConstructionScript
  (|CallParentFunction))